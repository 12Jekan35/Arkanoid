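; Base Arkanoid brick Blueprint that loses endurance when hit by a BP_Ball and destroys itself when none remains.
; Construction rolls a random endurance up to MaxEndurance and creates a dynamic material instance on the cube.
; SetEndurance caps the value and updates the material's Color parameter to show remaining endurance.
; It finds BP_CubeManager on BeginPlay and untracks itself from it when destroyed.
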(event EventDestroyed
  (Default|UntrackCube (Variables|Default|GetCubeManager) self))

(event EventBeginPlay
  (bind _returnvalue (Actor|GetActorOfClass "/Game/Arkanoid/Blueprints/Core/BP_CubeManager.BP_CubeManager_C"))
  (Variables|Default|SetCubeManager _returnvalue))

(event Collision|EventHit
  (params (MyComp :type Primitive%20Component%20Object%20Reference) (Other :type Actor%20Object%20Reference) (OtherComp :type Primitive%20Component%20Object%20Reference) (bSelfMoved :type Boolean) (HitLocation :type Vector :default "0, 0, 0") (HitNormal :type Vector :default "0, 0, 0") (NormalImpulse :type Vector :default "0, 0, 0") (Hit :type Hit%20Result%20Structure%20%28by%20ref%29))
  (Utilities|Casting|CastToBP_Ball Other)
  (bind _result (Math|Integer|DecrementInt (Variables|Default|GetEndurance))
    (:%20%20
      (bind _result_2 (CallFunction|SetEndurance _result))
      (if (> _result_2 0)
        (Development|PrintString (Utilities|String|Append "Endurance: " (Utilities|String|ToString(Integer) (Variables|Default|GetEndurance))))
        (else
          (Development|PrintString "Block is destroyed!")
          (Actor|DestroyActor))))))

(fn ConstructionScript
  (bind _returnvalue (Rendering|Material|CreateDynamicMaterialInstance (Variables|Default|GetCube) 0 (Variables|Default|GetMaterialInstance) "None" :!class /Script/Engine.PrimitiveComponent))
  (bind _output_get (Variables|Default|SetCurrentMaterial _returnvalue))
  (Rendering|Material|SetMaterial (Variables|Default|GetCube) 0 _output_get)
  (CallFunction|SetEndurance (Math|Random|RandomIntegerinRange 1 (Variables|Default|GetMaxEndurance))))

(fn SetEndurance
  (params (Value :type Integer))
  (bind _output_get (Variables|Default|SetEndurance (Math|Integer|Min(Integer) Value (Variables|Default|GetMaxEndurance))))
  (Rendering|Material|SetVectorParameterValue (Variables|Default|GetCurrentMaterial) "Color" (Utilities|Select :Index _output_get :Option%200 "" :Option%201 "(R=1.000000,G=0.000000,B=0.000000,A=1.000000)" :Option%202 "(R=1.000000,G=0.500000,B=0.000000,A=1.000000)" :Option%203 "(R=1.000000,G=1.000000,B=0.000000,A=1.000000)" :Option%204 "(R=0.500000,G=1.000000,B=0.000000,A=1.000000)" :Option%205 "(R=0.000000,G=1.000000,B=0.000000,A=1.000000)") :!class /Script/Engine.MaterialInstanceDynamic)
  (return (Variables|Default|GetEndurance)))