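; Manager for an Arkanoid game that keeps track of the balls in play.
; TrackNewBall adds balls to TrackedBalls, and DeleteBall casts a destroyed actor to BP_Ball and passes it to UntrackBall.
; UntrackBall removes the ball and calls CallBallsIsEmpty once none remain.
; A separate TrackedBallsIsEmpty event only prints a win message, with no binding to that call shown here.
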(event Custom|DeleteBall
  (params (DestroyedActor :type Actor%20Object%20Reference))
  (bind _asbp_ball (Utilities|Casting|CastToBP_Ball DestroyedActor))
  (CallFunction|UntrackBall _asbp_ball))

(event Custom|TrackedBallsIsEmpty
  (Development|PrintString "You're win!"))

(event EventBeginPlay)

(event Collision|EventActorBeginOverlap
  (params (OtherActor :type Actor%20Object%20Reference)))

(event EventTick
  (params (DeltaSeconds :type Float%20%28single-precision%29)))

(fn ConstructionScript)

(fn TrackNewBall
  (params (Ball :type BP%20Ball%20Object%20Reference))
  (Utilities|Array|Add (Variables|Default|GetTrackedBalls) Ball))

(fn UntrackBall
  (params (Ball :type BP%20Ball%20Object%20Reference))
  (Utilities|Array|RemoveItem (Variables|Default|GetTrackedBalls) Ball)
  (if (Utilities|Array|IsEmpty (Variables|Default|GetTrackedBalls))
    (Default|CallBallsIsEmpty)))