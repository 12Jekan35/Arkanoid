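; BP_CubeManager spawns and tracks the grid of cubes for an Arkanoid level.
; On BeginPlay it optionally randomizes grid size and spacing, scaling counts against spacing, then spawns a random CubeVariants class in each cell, offset from its own location.
; UntrackCube removes cubes from CubeList and fires CubesIsEmpty when none remain.
; A debug mesh preview in the construction script is disconnected.
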(event EventBeginPlay
  (bind _returnvalue (Transformation|GetActorLocation))
  (bind _padding (Variables|Default|GetPadding))
  (CallFunction|InitializeParameters (Variables|Default|GetbRandomParams))
  (for _index (range 0 (- (Variables|Default|GetX) 1))
    (for _index_2 (range 0 (- (Variables|Default|GetY) 1))
      (bind _returnvalue_2 (Game|SpawnActorfromClass (.OutItem (Utilities|Array|Random (Variables|Default|GetCubeVariants))) (Math|Transform|MakeTransform (Math|Vector|MakeVector (- (.x _returnvalue) (* _index (.x _padding))) (- (.y _returnvalue) (* _index_2 (.y _padding))) 5e+01)) "Undefined" 0 0))
      (Utilities|Array|Add (Variables|Default|GetCubeList) _returnvalue_2))))

(event EventTick
  (params (DeltaSeconds :type Float%20%28single-precision%29)))

(fn ConstructionScript)

(fn DebugLocationCubes)

(fn InitializeParameters
  (params (Random :type Boolean))
  (bind _returnvalue (Math|Random|RandomIntegerinRange 1 2))
  (if Random
    (bind _output_get (LocalVariables|SetXModifier _returnvalue))
    (bind _output_get_2 (LocalVariables|SetYModifier _returnvalue))
    (Variables|Default|SetPadding (Math|Vector|MakeVector (* _output_get 1e+02) (* _output_get_2 1e+02) 0.0))
    (Variables|Default|SetX (Math|Random|RandomIntegerinRange 1 (/ 8 (LocalVariables|GetXModifier))))
    (Variables|Default|SetY (Math|Random|RandomIntegerinRange (/ 18 (LocalVariables|GetYModifier)) (/ 24 (LocalVariables|GetYModifier)))))
  (return))

(fn UntrackCube
  (params (Cube :type BP%20Cube%20Base%20Object%20Reference))
  (bind _cubelist (Variables|Default|GetCubeList))
  (Utilities|Array|RemoveItem _cubelist Cube)
  (if (Utilities|Array|IsEmpty _cubelist)
    (Default|CallCubesIsEmpty)))