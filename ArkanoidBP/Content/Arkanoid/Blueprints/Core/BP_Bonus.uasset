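; Arkanoid bonus pickup that moves along negative X and, when it overlaps the platform, applies its effect and destroys itself.
; The construction script randomly picks one of two types and tints a dynamic sphere material to match.
; BeginPlay binds that type's effect to the MakeEffect dispatcher.
; MultiplyBalls spawns an extra ball at each ball tracked by BP_BallManager, while MakeBalls spawns three diverging balls just ahead of the platform.
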(event Custom|MultiplyBalls
  (params (Actor :type Actor%20Object%20Reference))
  (bind _returnvalue (Actor|GetActorOfClass "/Game/Arkanoid/Blueprints/Core/BP_BallManager.BP_BallManager_C"))
  (bind _output_get (Variables|Default|SetCountBalls (Utilities|Array|Length (Variables|/Game/Arkanoid/Blueprints/Core/BP_BallManager.BP_BallManager_C|GetTrackedBalls _returnvalue))))
  (for _index (range 0 (- _output_get 1))
    (bind _returnvalue_2 (Game|SpawnActorfromClass "/Game/Arkanoid/Blueprints/Core/BP_Ball.BP_Ball_C" (Transformation|GetActorTransform (Utilities|Array|Get(acopy) (Variables|/Game/Arkanoid/Blueprints/Core/BP_BallManager.BP_BallManager_C|GetTrackedBalls _returnvalue) _index)) "Undefined" 0 0))
    (Variables|/Game/Arkanoid/Blueprints/Core/BP_Ball.BP_Ball_C|SetDirection _returnvalue_2 (Utilities|Select :Index (Math|Random|RandomIntegerinRange 0 2) :Option%200 "1.000000,1.000000,0.000000" :Option%201 "1.000000,-1.000000,0.000000" :Option%202 "1.000000,0.000000,0.000000"))))

(event Custom|MakeBalls
  (params (Actor :type Actor%20Object%20Reference))
  (bind _returnvalue (Transformation|GetActorTransform Actor))
  (bind (_location _rotation) (Math|Transform|BreakTransform _returnvalue))
  (for _index (range 0 2)
    (bind _returnvalue_2 (Game|SpawnActorfromClass "/Game/Arkanoid/Blueprints/Core/BP_Ball.BP_Ball_C" (Math|Transform|MakeTransform (Math|Vector|MakeVector (+ (.x _location) 1e+02) (.y _location) (.z _location)) _rotation) "Undefined" 0 0))
    (Variables|/Game/Arkanoid/Blueprints/Core/BP_Ball.BP_Ball_C|SetDirection _returnvalue_2 (Utilities|Select :Index _index :Option%200 "1.000000,1.000000,0.000000" :Option%201 "1.000000,-1.000000,0.000000" :Option%202 "1.000000,0.000000,0.000000"))))

(event Collision|EventActorBeginOverlap
  (params (OtherActor :type Actor%20Object%20Reference))
  (bind _asbp_platform (Utilities|Casting|CastToBP_Platform OtherActor))
  (Default|CallMakeEffect _asbp_platform)
  (Actor|DestroyActor))

(event EventBeginPlay
  (EventDispatchers|BindEventtoMakeEffect (Utilities|Select :Index (Variables|Default|GetIndex) :Option%200 (delegate Custom|MultiplyBalls) :Option%201 (delegate Custom|MakeBalls))))

(event EventTick
  (params (DeltaSeconds :type Float%20%28single-precision%29))
  (Transformation|AddActorWorldOffset (Math|Vector|MakeVector (* DeltaSeconds (Variables|Default|GetSpeed) -1.0) 0.0 0.0) true))

(fn ConstructionScript
  (bind _returnvalue (Rendering|Material|CreateDynamicMaterialInstance (Variables|Default|GetSphere) 0 "/Game/Arkanoid/Materials/Bonus/M_Bonus.M_Bonus" "None" :!class /Script/Engine.PrimitiveComponent))
  (bind _output_get (Variables|Default|SetMaterial _returnvalue))
  (bind _output_get_2 (Variables|Default|SetIndex (Math|Random|RandomIntegerinRange 0 1)))
  (Rendering|Material|SetVectorParameterValue _output_get "RGBA" (Utilities|Select :Index _output_get_2 :Option%200 "(R=1.000000,G=0.635954,B=0.000000,A=0.300000)" :Option%201 "(R=1.000000,G=0.000000,B=1.000000,A=0.300000)") :!class /Script/Engine.MaterialInstanceDynamic))