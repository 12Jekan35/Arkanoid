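; BP_Ball is the Arkanoid ball actor, which moves itself and bounces off whatever it hits.
; Each Tick it applies a swept X/Y offset from Direction and Speed; on a blocking hit it reflects Direction about the hit normal and raises Speed up to a cap, printing the new value.
; It registers with BP_BallManager on BeginPlay and untracks itself when destroyed.
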(event EventBeginPlay
  (bind _returnvalue (Actor|GetActorOfClass "/Game/Arkanoid/Blueprints/Core/BP_BallManager.BP_BallManager_C"))
  (bind _output_get (Variables|Default|SetBallManager _returnvalue))
  (Default|TrackNewBall _output_get self))

(event Collision|EventActorBeginOverlap
  (params (OtherActor :type Actor%20Object%20Reference)))

(event EventTick
  (params (DeltaSeconds :type Float%20%28single-precision%29))
  (bind _sweephitresult (Transformation|AddActorWorldOffset (Math|Vector|MakeVector (.x (* (* DeltaSeconds (Variables|Default|GetSpeed)) (Variables|Default|GetDirection))) (.y (* (* DeltaSeconds (Variables|Default|GetSpeed)) (Variables|Default|GetDirection))) 0.0) true))
  (if (.bBlockingHit (Collision|BreakHitResult _sweephitresult))
    (Variables|Default|SetDirection (Math|Vector|GetReflectionVector (Variables|Default|GetDirection) (.Normal (Collision|BreakHitResult _sweephitresult))))
    (bind _output_get (Variables|Default|SetSpeed (Math|Float|Min(Float) (+ (Variables|Default|GetSpeed) (Variables|Default|GetSpeedModifier)) (Variables|Default|GetMaxSpeed))))
    (Development|PrintString (Utilities|String|ToString(Float) _output_get))))

(event EventDestroyed
  (Default|UntrackBall (Variables|Default|GetBallManager) self))

(fn ConstructionScript)