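; Arkanoid game mode that decides when the match is won or lost.
; On BeginPlay it finds the ball and cube managers and binds Lose to running out of balls and Win to clearing all cubes.
; Both outcomes focus the player controller's widget, fire OnLose or OnWin and pause the game.
; Lose switches input to UI only, while Win uses Game and UI.
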(event Custom|Lose
  ;[1 1 1] Lose
  (bind _asbp_player_controller (Utilities|Casting|CastToBP_PlayerController (Game|GetPlayerController 0)))
  (Input|SetInputModeUIOnly _asbp_player_controller (Variables|/Game/Arkanoid/Blueprints/Player/BP_PlayerController.BP_PlayerController_C|GetWidget _asbp_player_controller) "DoNotLock" false)
  (Default|CallOnLose)
  (Game|SetGamePaused true))

(event Custom|Win
  ;[1 1 1] Win
  (bind _asbp_player_controller (Utilities|Casting|CastToBP_PlayerController (Game|GetPlayerController 0)))
  (Input|SetInputModeGameandUI _asbp_player_controller (Variables|/Game/Arkanoid/Blueprints/Player/BP_PlayerController.BP_PlayerController_C|GetWidget _asbp_player_controller) "DoNotLock" false false)
  (Default|CallOnWin)
  (Game|SetGamePaused true))

(event EventBeginPlay
  (bind _returnvalue (Actor|GetActorOfClass "/Game/Arkanoid/Blueprints/Core/BP_BallManager.BP_BallManager_C"))
  (bind _output_get (Variables|Default|SetBallManager _returnvalue))
  (EventDispatchers|BindEventtoBallsIsEmpty _output_get (delegate Custom|Lose))
  (bind _returnvalue_2 (Actor|GetActorOfClass "/Game/Arkanoid/Blueprints/Core/BP_CubeManager.BP_CubeManager_C"))
  (bind _output_get_2 (Variables|Default|SetCubeManager _returnvalue_2))
  (EventDispatchers|BindEventtoCubesIsEmpty _output_get_2 (delegate Custom|Win)))

(fn ConstructionScript)