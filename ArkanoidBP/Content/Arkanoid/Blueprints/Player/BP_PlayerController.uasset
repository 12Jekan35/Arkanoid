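; Player controller for the Arkanoid game that drives up to two paddle platforms and creates the game widget on BeginPlay.
; The first possessed BP_Platform is stored as Platform, and a later possession fills Platform2 while the first remains valid.
; Separate input axes move each stored platform, so one controller serves both local players.
; The Menu input fires the OpenCloseMenu event dispatcher.
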(event EventBeginPlay
  (bind _returnvalue (Game|ConstructObjectfromClass "/Game/Arkanoid/Blueprints/UI/BPW_Game.BPW_Game_C"))
  (bind _output_get (Variables|Default|SetWidget _returnvalue))
  (UserInterface|Viewport|AddtoViewport _output_get 0))

(event EventPossess
  (params (PossessedPawn :type Pawn%20Object%20Reference))
  (bind _asbp_platform (Utilities|Casting|CastToBP_Platform PossessedPawn))
  (if (Utilities|IsValid (Variables|Default|GetPlatform))
    (Variables|Default|SetPlatform2 _asbp_platform)
    (else
      (Variables|Default|SetPlatform _asbp_platform))))

(event Input|ActionEvents|InputActionMenu
  (params (Key :type Key%20Structure :default "None"))
  (:Pressed
    (Default|CallOpenCloseMenu)))

(event Input|AxisEvents|InputAxisMoveRight
  (params (AxisValue :type Float%20%28single-precision%29))
  (bind _platform (Variables|Default|GetPlatform))
  (if (Utilities|IsValid _platform)
    (Default|MakeMoveRight _platform AxisValue)))

(event Input|AxisEvents|InputAxisMoveRight2Player
  (params (AxisValue :type Float%20%28single-precision%29))
  (bind _platform2 (Variables|Default|GetPlatform2))
  (if (Utilities|IsValid _platform2)
    (Default|MakeMoveRight _platform2 AxisValue)))

(fn ConstructionScript)